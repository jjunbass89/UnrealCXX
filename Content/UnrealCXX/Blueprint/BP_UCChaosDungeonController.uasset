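; BP_UCChaosDungeonController is the Chaos Dungeon controller that drives the HUD and reacts to score, game and portal events.
; BeginPlay creates WBP_HUD and caches its dungeon, death and clear dialogs.
; Score changes update the percentage text, while game clear and game over show their dialogs.
; Hiding the death dialog triggers Revival through a visibility binding, and entering a portal opens the ChaosDungeon1 level.
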(event Custom|OnDeadDlgVisibilityChanged
  (params (InVisibility :type ESlateVisibility%20Enum :default "Visible"))
  (if (Utilities|Enum|Equal(Enum) InVisibility "Hidden")
    (Class|UCChaosDungeonController|Revival)))

(event EventBeginPlay
  (bind _returnvalue (UserInterface|CreateWidget "/Game/UnrealCXX/UI/WBP_HUD.WBP_HUD_C"))
  (UserInterface|Viewport|AddtoViewport _returnvalue 0)
  (Variables|Default|SetWBP%20Chaos%20Dungeon%20Dlg (Variables|/Game/UnrealCXX/UI/WBP_HUD.WBP_HUD_C|GetWBP_ChaosDungeonDlg _returnvalue))
  (Variables|Default|SetWBP%20Dead%20Dlg (Variables|/Game/UnrealCXX/UI/WBP_HUD.WBP_HUD_C|GetWBP_DeadDlg _returnvalue))
  (Variables|Default|SetWBP%20Clear%20Dlg (Variables|/Game/UnrealCXX/UI/WBP_HUD.WBP_HUD_C|GetWBP_ClearDlg _returnvalue))
  (EventDispatchers|BindEventtoOnVisibilityChanged (Variables|/Game/UnrealCXX/UI/WBP_HUD.WBP_HUD_C|GetWBP_DeadDlg _returnvalue) (delegate Custom|OnDeadDlgVisibilityChanged)))

(event EventTick
  (params (DeltaSeconds :type Float%20%28single-precision%29)))

(event EventOnScoreChanged
  (params (NewScore :type Integer))
  (Rendering|Components|TextRender|SetText (Variables|/Game/UnrealCXX/UI/WBP_ChaosDungeonDlg.WBP_ChaosDungeonDlg_C|GetPercentTxt (Variables|Default|GetWBP%20Chaos%20Dungeon%20Dlg)) (Utilities|Text|FormatText "{Percentage} %" (Utilities|Text|ToText(Float) (Math|Conversions|ToFloat(Integer) NewScore) "HalfToEven"))))

(event EventOnGameClear
  (Widget|SetVisibility (Variables|Default|GetWBP%20Clear%20Dlg) "Visible"))

(event EventOnGameOver
  (Widget|SetVisibility (Variables|Default|GetWBP%20Dead%20Dlg) "Visible"))

(event EventOnEnterPortal
  (params (NewScore :type Integer))
  (Game|OpenLevel(byName) "ChaosDungeon1"))

(fn ConstructionScript)